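; Floor actor that responds to controller trace events, showing a separate ring marker for the left and right controllers.
; Object hit and leave events toggle the matching ring's visibility, while trace movement snaps it to the hit location, oriented along the surface normal.
; Component hit and leave both only unhide the left ring because their branch is hard-coded true.
; Activate handlers are stubs returning false, and the event graph is empty.
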(event EventBeginPlay)

(event Collision|EventActorBeginOverlap
  (params (OtherActor :type Actor%20Object%20Reference)))

(event EventTick
  (params (DeltaSeconds :type Float%20%28single-precision%29)))

(fn ConstructionScript)

(fn TraceActivateDown
  (params (Hit :type Hit%20Result%20Structure) (Instigator :type Pawn%20Object%20Reference))
  (return false))

(fn TraceActivateUp
  (params (Hit :type Hit%20Result%20Structure) (Instigator :type Pawn%20Object%20Reference))
  (return false))

(fn TraceHitComponent
  (params (Hit :type Hit%20Result%20Structure) (Component :type Primitive%20Component%20Object%20Reference))
  (if true
    (Development|SetHiddeninGame (Variables|Default|GetLeftRing) false false)
    (return false)
    (else
      (Development|SetHiddeninGame (Variables|Default|GetRightRing) false false))))

(fn TraceHitObject
  (params (Hit :type Hit%20Result%20Structure) (IsLeftController :type Boolean))
  (if IsLeftController
    (Development|SetHiddeninGame (Variables|Default|GetLeftRing) false false)
    (return false)
    (else
      (Development|SetHiddeninGame (Variables|Default|GetRightRing) false false)
      (return false))))

(fn TraceLeaveComponent
  (params (Component :type Primitive%20Component%20Object%20Reference) (Hit :type Hit%20Result%20Structure))
  (if true
    (Development|SetHiddeninGame (Variables|Default|GetLeftRing) false false)
    (return false)
    (else
      (Development|SetHiddeninGame (Variables|Default|GetRightRing) false false))))

(fn TraceLeaveObject
  (params (Hit :type Hit%20Result%20Structure) (IsLeftController :type Boolean))
  (if IsLeftController
    (Development|SetHiddeninGame (Variables|Default|GetLeftRing) true false)
    (return false)
    (else
      (Development|SetHiddeninGame (Variables|Default|GetRightRing) true false)
      (return false))))

(fn TraceMove
  (params (Hit :type Hit%20Result%20Structure%20%28by%20ref%29) (IsLeftController :type Boolean))
  (bind (_bblockinghit _binitialoverlap _time _distance _location _impactpoint _normal) (Collision|BreakHitResult Hit))
  (bind _returnvalue (Math|Rotator|MakeRotfromX _normal))
  (if IsLeftController
    (Transformation|SetWorldLocationAndRotation (Variables|Default|GetLeftRing) _location _returnvalue false false)
    (return false)
    (else
      (Transformation|SetWorldLocationAndRotation (Variables|Default|GetRightRing) _location _returnvalue false false)
      (return false))))