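; Test cube that reacts to controller traces by restarting a color fade on its material.
; Tick raises an unclamped alpha by a fixed per-frame step, lerping the Color parameter from black toward magenta.
; TraceHitObject and TraceActivateDown reset the alpha, snapping the cube back to black.
; The other trace handlers, including teleport, are stubs, and every handler returns false.
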(event EventBeginPlay
  (Rendering|Material|SetVectorParameterValueonMaterials (Variables|Default|GetCube) "Color" "0.500000,0.500000,0.500000"))

(event Collision|EventActorBeginOverlap
  (params (OtherActor :type Actor%20Object%20Reference)))

(event EventTick
  (params (DeltaSeconds :type Float%20%28single-precision%29))
  (bind _output_get (Variables|Default|SetColorTransitionAlpha (+ (Variables|Default|GetColorTransitionAlpha) 0.01)))
  (Rendering|Material|SetVectorParameterValueonMaterials (Variables|Default|GetCube) "Color" (Math|Vector|Lerp(Vector) "0, 0, 0" "1.000000,0.000000,1.000000" _output_get)))

(fn ConstructionScript
  (Rendering|Material|SetVectorParameterValueonMaterials (Variables|Default|GetCube) "Color" "0, 0, 0"))

(fn TraceActivateDown
  (params (Hit :type Hit%20Result%20Structure) (Instigator :type Pawn%20Object%20Reference))
  (Variables|Default|SetColorTransitionAlpha 0.0)
  (return false))

(fn TraceActivateTeleportDown
  (params (Hit :type Hit%20Result%20Structure) (Instigator :type Pawn%20Object%20Reference))
  (return false))

(fn TraceActivateTeleportUp
  (params (Hit :type Hit%20Result%20Structure) (Instigator :type Pawn%20Object%20Reference))
  (return false))

(fn TraceActivateUp
  (params (Hit :type Hit%20Result%20Structure) (Instigator :type Pawn%20Object%20Reference))
  (return false))

(fn TraceHitComponent
  (params (Hit :type Hit%20Result%20Structure) (Component :type Primitive%20Component%20Object%20Reference))
  (return false))

(fn TraceHitObject
  (params (Hit :type Hit%20Result%20Structure) (IsLeftController :type Boolean))
  (Variables|Default|SetColorTransitionAlpha 0.0)
  (return false))

(fn TraceLeaveComponent
  (params (Component :type Primitive%20Component%20Object%20Reference) (Hit :type Hit%20Result%20Structure))
  (return false))

(fn TraceLeaveObject
  (params (Hit :type Hit%20Result%20Structure) (IsLeftController :type Boolean))
  (return false))

(fn TraceMove
  (params (Hit :type Hit%20Result%20Structure%20%28by%20ref%29) (IsLeftController :type Boolean))
  (return false))